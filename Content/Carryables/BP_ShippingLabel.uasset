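; BP_ShippingLabel is a carryable shipping label Blueprint that can be applied to wrapped presents.
; When interacted with alongside a carried object, it casts that object to BP_WrappedPresent and forwards Interact to it, passing itself; other objects are ignored.
; On BeginPlay it runs the parent logic, then prints the name of the Item from its LetterData class defaults.
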(event EventBeginPlay
  (|CallParentFunction)
  (Development|PrintString (Utilities|GetObjectName (.Item (Utilities|GetClassDefaults (Variables|Default|GetLetterData))))))

(event Collision|EventActorBeginOverlap
  (params (OtherActor :type Actor%20Object%20Reference))
  (|CallParentFunction OtherActor) ; This node is disabled and will not be called.\nDrag off pins to build functionality.
)

(event EventTick
  (params (DeltaSeconds :type Float%20%28single-precision%29))
  (|CallParentFunction DeltaSeconds) ; This node is disabled and will not be called.\nDrag off pins to build functionality.
)

(event EventInteract
  (params (CarriedObject :type Actor%20Object%20Reference))
  (bind _asbp_wrapped_present (Utilities|Casting|CastToBP_WrappedPresent CarriedObject))
  (Default|Interact _asbp_wrapped_present self))

(fn ConstructionScript
  (|CallParentFunction))