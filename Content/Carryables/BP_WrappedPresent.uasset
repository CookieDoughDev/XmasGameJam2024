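; BP_WrappedPresent is a wrapped gift in the Carryables folder that accepts a carried shipping label.
; Its label component starts hidden; Interact with a BP_ShippingLabel reveals it, copies that label's LetterData, then has the parent BP_Player drop the carried label before destroying it.
; Names of the wrapped gift and the letter's item are printed for debugging.
; Unconnected logic for randomizing the present mesh and offsetting the label never runs.
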(event EventBeginPlay
  (|CallParentFunction)
  (Rendering|SetVisibility (Variables|Default|GetShippingLabel) false false)
  (Development|PrintString (Utilities|GetObjectName (Variables|Default|GetWrappedGift))))

(event Collision|EventActorBeginOverlap
  (params (OtherActor :type Actor%20Object%20Reference))
  (|CallParentFunction OtherActor) ; This node is disabled and will not be called.\nDrag off pins to build functionality.
)

(event EventTick
  (params (DeltaSeconds :type Float%20%28single-precision%29))
  (|CallParentFunction DeltaSeconds) ; This node is disabled and will not be called.\nDrag off pins to build functionality.
)

(event EventInteract
  (params (CarriedObject :type Actor%20Object%20Reference))
  (bind _asbp_shipping_label (Utilities|Casting|CastToBP_ShippingLabel CarriedObject))
  (Rendering|SetVisibility (Variables|Default|GetShippingLabel) true false)
  (bind _output_get (Variables|Default|SetLetterData (Variables|/Game/Carryables/BP_ShippingLabel.BP_ShippingLabel_C|GetLetterData _asbp_shipping_label)))
  (Development|PrintString (Utilities|GetObjectName (.Item (Utilities|GetClassDefaults _output_get))))
  (bind _asbp_player (Utilities|Casting|CastToBP_Player (Actor|GetParentActor CarriedObject)))
  (Default|DropObject _asbp_player)
  (Actor|DestroyActor CarriedObject))

(fn ConstructionScript
  (|CallParentFunction))