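; AC_Container is a container component that holds an Actor by attaching it to a Slot scene component.
; PutActor attaches the given Actor's root component to Slot, snapping location, rotation and scale.
; GetContainedActor keeps no stored reference, instead returning the owner of Slot's first child component.
; BeginPlay checks that Slot is valid but does nothing with the result, as the missing-slot warning print is unconnected.
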(event EventBeginPlay
  (Utilities|IsValid (Variables|Default|GetSlot)))

(fn PutActor
  (params (Actor :type Actor%20Object%20Reference))
  (Transformation|AttachComponentToComponent (Variables|/Script/Engine.Actor|GetRootComponent Actor) (Variables|Default|GetSlot) "None" "SnapToTarget" "SnapToTarget" "SnapToTarget" true))

(fn GetContainedActor
  (bind _slot (Variables|Default|GetSlot))
  (bind _returnvalue (Components|GetChildComponent _slot 0))
  (Utilities|IsValid _returnvalue
    (:Is%20Valid
      (return (Components|GetOwner _returnvalue)))))