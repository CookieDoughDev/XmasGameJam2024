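; AC_Interact is an actor component that picks which nearby interactable its owner should target.
; GetNearestInteractable filters a given list of actors down to those implementing BPI_Interactable.
; It then returns the filtered actor closest to the owner's location, or nothing when none qualify.
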(fn GetNearestInteractable
  (params (Interactables :type Array%20of%20Actor%20Object%20References))
  ;[0.125 0.125 0.125] Only include actors with interactable interface
  (for _array_element Interactables
    (if (Utilities|DoesObjectImplementInterface _array_element "/Game/Core/Interfaces/BPI_Interactable.BPI_Interactable_C")
      (Utilities|Array|Add (LocalVariables|GetFiltered%20Interactables) _array_element)))
  ;[0.125 0.125 0.125] Are any interactables nearby?
  (if (Utilities|Array|IsNotEmpty (LocalVariables|GetFiltered%20Interactables))
    ;[0.125 0.125 0.125] Get the nearest Interactable
    (return (.ReturnValue (Actor|FindNearestActor (Transformation|GetActorLocation (Components|GetOwner)) (LocalVariables|GetFiltered%20Interactables))))
    (else
      (return 0))))