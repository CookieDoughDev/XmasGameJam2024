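; Player controller that handles drop-in and drop-out of a second local player.
; BeginPlay adds the IMC_P1 Enhanced Input mapping context to player 0's subsystem.
; IA_JoystickAny creates local player 1 and passes its controller ID to its pawn through BP_Player's AssignPlayer.
; IA_Disconnect removes the player at index 1 and destroys its pawn.
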(event Input|EnhancedActionEvents|EnhancedInputActionIA_Disconnect
  (params (ActionValue :type Boolean) (ElapsedSeconds :type Float%20%28double-precision%29) (TriggeredSeconds :type Float%20%28double-precision%29) (InputAction :type Input%20Action%20Object%20Reference :default "/Game/Core/Input/Actions/IA_Disconnect.IA_Disconnect"))
  (:Started
    (Class|GameplayStatics|RemovePlayer (Game|GetPlayerController 1) true)))

(event Input|EnhancedActionEvents|EnhancedInputActionIA_JoystickAny
  (params (ActionValue :type Boolean) (ElapsedSeconds :type Float%20%28double-precision%29) (TriggeredSeconds :type Float%20%28double-precision%29) (InputAction :type Input%20Action%20Object%20Reference :default "/Game/Core/Input/Actions/IA_JoystickAny.IA_JoystickAny"))
  (:Started
    (bind _returnvalue (Class|GameplayStatics|CreatePlayer 1))
    (Utilities|IsValid _returnvalue
      (:Is%20Valid
        (bind _asbp_player (Utilities|Casting|CastToBP_Player (Pawn|GetControlledPawn _returnvalue)))
        (Default|AssignPlayer _asbp_player (Class|GameplayStatics|GetPlayerControllerID _returnvalue))))))

(event EventBeginPlay
  (Input|AddMappingContext (PlayerController|LocalPlayerSubsystems|GetEnhancedInputLocalPlayerSubsystem (Game|GetPlayerController 0)) "/Game/Core/Input/IMC_P1.IMC_P1" 0 "(bIgnoreAllPressedKeysUntilRelease=True,bForceImmediately=False,bNotifyUserSettings=False)"))

(fn ConstructionScript)