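; BP_Letter is a letter actor that shows a widget component while the player overlaps its static mesh.
; The widget starts hidden and becomes visible when a BP_Player begins overlapping the mesh.
; Any end overlap hides it again, with no check on which actor left.
; The construction script randomly picks one of two mail meshes, so placed letters vary in look.
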(event OnComponentBeginOverlap(StaticMesh)
  (params (OverlappedComponent :type Primitive%20Component%20Object%20Reference) (OtherActor :type Actor%20Object%20Reference) (OtherComp :type Primitive%20Component%20Object%20Reference) (OtherBodyIndex :type Integer) (bFromSweep :type Boolean) (SweepResult :type Hit%20Result%20Structure%20%28by%20ref%29))
  (Utilities|Casting|CastToBP_Player OtherActor)
  (Rendering|SetVisibility (Variables|Default|GetWidget) true false))

(event OnComponentEndOverlap(StaticMesh)
  (params (OverlappedComponent :type Primitive%20Component%20Object%20Reference) (OtherActor :type Actor%20Object%20Reference) (OtherComp :type Primitive%20Component%20Object%20Reference) (OtherBodyIndex :type Integer))
  (Rendering|SetVisibility (Variables|Default|GetWidget) false false))

(event EventBeginPlay
  (Rendering|SetVisibility (Variables|Default|GetWidget) false false))

(fn ConstructionScript
  (bind _staticmesh (Variables|Default|GetStaticMesh))
  (if (Math|Random|RandomBool)
    (Components|StaticMesh|SetStaticMesh _staticmesh "/Game/Low_Poly_Viking_Interiors/Models/Props/Library/SM_Book_09_Mail_01.SM_Book_09_Mail_01")
    (else
      (Components|StaticMesh|SetStaticMesh _staticmesh "/Game/Low_Poly_Viking_Interiors/Models/Props/Library/SM_Book_09_Mail_03.SM_Book_09_Mail_03"))))