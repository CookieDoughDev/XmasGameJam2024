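; BP_Lamp_02 is a configurable lamp prop from the Low Poly Viking Interiors pack, combining a lamp mesh, spotlight, particles and lightshaft mesh.
; Its construction script applies exposed variables to the spotlight's intensity and color and the mesh's material, and toggles visibility of the particles and lightshaft.
; The event graph is empty, so the actor has no runtime logic.
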(event EventBeginPlay)

(event Collision|EventActorBeginOverlap
  (params (OtherActor :type Actor%20Object%20Reference)))

(event EventTick
  (params (DeltaSeconds :type Float%20%28single-precision%29)))

(fn ConstructionScript
  (bind _spotlight_0 (Variables|Default|GetSpotlight_0))
  (Rendering|Components|Light|SetIntensity _spotlight_0 (Variables|Default|GetLight_Intensity))
  (Rendering|Components|Light|SetLightColor _spotlight_0 (Variables|Default|GetLight_Color) true)
  (Rendering|Material|SetMaterial (Variables|Default|GetSM_Lamp_02) 0 (Variables|Default|GetMaterial))
  (Rendering|SetVisibility (Variables|Default|GetParticles) (Variables|Default|GetParticle) true)
  (Rendering|SetVisibility (Variables|Default|GetSM_Lightshaft) (Variables|Default|GetLightshaft) false))