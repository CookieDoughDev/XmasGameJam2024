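; BP_BaseStation is a station, apparently a base class, that shows on-site prompts when a player approaches.
; It hides its InputPrompt, Description, Showcase and Requirement components on BeginPlay and when any overlap ends.
; On overlap by a player-controlled instigator, it reveals all but Showcase, then hides Requirement if the BP_Player's carried object class matches RequiredItem.
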(event Collision|EventActorBeginOverlap
  (params (OtherActor :type Actor%20Object%20Reference))
  (bind _instigator (Variables|/Script/Engine.Actor|GetInstigator OtherActor))
  (Utilities|IsValid _instigator
    (:Is%20Valid
      (Utilities|Casting|CastToPlayerController (Pawn|GetController _instigator))
      (Rendering|SetVisibility (Variables|Default|GetInputPrompt) true false)
      (bind _asbp_player (Utilities|Casting|CastToBP_Player _instigator))
      (if (== (Utilities|GetClass (Default|GetCarriedObject _asbp_player)) (Variables|Default|GetRequiredItem))
        (Rendering|SetVisibility (Variables|Default|GetRequirement) false false)))))

(event Collision|EventActorEndOverlap
  (params (OtherActor :type Actor%20Object%20Reference))
  (Rendering|SetVisibility (Variables|Default|GetInputPrompt) false false))

(event EventBeginPlay
  (Rendering|SetVisibility (Variables|Default|GetInputPrompt) false false))

(fn ConstructionScript)