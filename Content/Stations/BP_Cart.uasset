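; BP_Cart is a station that receives wrapped presents and shows whether each holds the requested gift.
; When a BP_WrappedPresent overlaps its sphere, it compares the Item in the class defaults of the present's LetterData with the WrappedGift inside.
; Santa's flipbook switches to happy on a match or angry otherwise, then the present is destroyed.
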(event OnComponentBeginOverlap(Sphere)
  (params (OverlappedComponent :type Primitive%20Component%20Object%20Reference) (OtherActor :type Actor%20Object%20Reference) (OtherComp :type Primitive%20Component%20Object%20Reference) (OtherBodyIndex :type Integer) (bFromSweep :type Boolean) (SweepResult :type Hit%20Result%20Structure%20%28by%20ref%29))
  (bind _santa (Variables|Default|GetSanta))
  (bind _rendercomponent (Variables|/Script/Paper2D.PaperFlipbookActor|GetRenderComponent _santa))
  (bind _asbp_wrapped_present (Utilities|Casting|CastToBP_WrappedPresent OtherActor))
  (if (== (Utilities|GetClass _asbp_wrapped_present) "/Game/Carryables/BP_WrappedPresent.BP_WrappedPresent_C")
    (Utilities|FlowControl|Sequence
      (:then_0
        (if (== (.Item (Utilities|GetClassDefaults (Variables|/Game/Carryables/BP_WrappedPresent.BP_WrappedPresent_C|GetLetterData _asbp_wrapped_present))) (Variables|/Game/Carryables/BP_WrappedPresent.BP_WrappedPresent_C|GetWrappedGift _asbp_wrapped_present))
          (Sprite|SetFlipbook _rendercomponent "/Game/Santa/PF_HappySanta.PF_HappySanta")
          (else
            (Sprite|SetFlipbook _rendercomponent "/Game/Santa/PF_AngrySanta.PF_AngrySanta"))))
      (:then_1
        (Actor|DestroyActor OtherActor)))))

(fn ConstructionScript)