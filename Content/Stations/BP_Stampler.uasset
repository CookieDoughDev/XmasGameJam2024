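; BP_Stampler is a station Blueprint that reveals its Showcase component when interacted with using a carried object.
; Interact checks that the object and the actor it is attached to are valid, then passes a hard-wired true branch to show Showcase.
; A BP_Letter class check and an instigator controller lookup are present but unused, so the object's type is not checked.
; Nothing in the file hides Showcase again or performs any stamping.
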(event EventInteract
  (params (CarriedObject :type Actor%20Object%20Reference))
  (Utilities|IsValid CarriedObject
    (:Is%20Valid
      (Utilities|IsValid (Actor|GetAttachParentActor CarriedObject)
        (:Is%20Valid
          (if true
            (Rendering|SetVisibility (Variables|Default|GetShowcase) true false)))))))

(fn ConstructionScript
  (|CallParentFunction))