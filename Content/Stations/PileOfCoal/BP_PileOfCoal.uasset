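; BP_PileOfCoal is a station that hands a coal object to a player on interaction.
; Its begin-overlap event stores the most recent overlapping BP_Player as NearestPlayer, with no distance check or clearing here.
; Interact spawns a BP_Toy_Coal at that player's transform, if valid, and passes it to the player's TakeObject.
; No supply limit or cooldown is applied in this Blueprint.
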(event Collision|EventActorBeginOverlap
  (params (OtherActor :type Actor%20Object%20Reference))
  (|CallParentFunction OtherActor)
  (bind _asbp_player (Utilities|Casting|CastToBP_Player OtherActor))
  (Variables|Default|SetNearestPlayer _asbp_player))

(event EventInteract
  (params (CarriedObject :type Actor%20Object%20Reference))
  (bind _nearestplayer (Variables|Default|GetNearestPlayer))
  (Utilities|IsValid _nearestplayer
    (:Is%20Valid
      (bind _returnvalue (Game|SpawnActorfromClass "/Game/Toys/BP_Toy_Coal.BP_Toy_Coal_C" (Transformation|GetActorTransform _nearestplayer) "Undefined" "MultiplyWithRoot" 0 0))
      (Default|TakeObject _nearestplayer _returnvalue))))

(fn ConstructionScript
  (|CallParentFunction))