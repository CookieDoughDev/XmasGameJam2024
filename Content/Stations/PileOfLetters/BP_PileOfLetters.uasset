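; BP_PileOfLetters is an interactable station that hands out letters to players from a list of letter data.
; On actor overlap it stores an overlapping BP_Player as the nearest player.
; Interact spawns a BP_Letter at that player's transform, then moves the first LetterList entry onto it and has the player take it.
; The spawn precedes the empty-list check, so an empty pile still spawns a letter that is not handed over.
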(event Collision|EventActorBeginOverlap
  (params (OtherActor :type Actor%20Object%20Reference))
  (|CallParentFunction OtherActor)
  (bind _asbp_player (Utilities|Casting|CastToBP_Player OtherActor))
  (Variables|Default|SetNearestPlayer _asbp_player))

(event EventInteract
  (params (CarriedObject :type Actor%20Object%20Reference))
  (bind _nearestplayer (Variables|Default|GetNearestPlayer))
  (bind _letterlist (Variables|Default|GetLetterList))
  (Utilities|IsValid _nearestplayer
    (:Is%20Valid
      (bind _returnvalue (Game|SpawnActorfromClass "/Game/Letters/BP_Letter.BP_Letter_C" (Transformation|GetActorTransform _nearestplayer) "Undefined" "MultiplyWithRoot" 0 0))
      (if (Utilities|Array|IsNotEmpty _letterlist)
        (bind _output_get (Variables|/Game/Letters/BP_Letter.BP_Letter_C|SetLetterData _returnvalue (Utilities|Array|Get(acopy) _letterlist)))
        (Utilities|Array|RemoveItem _letterlist _output_get)
        (Default|TakeObject _nearestplayer _returnvalue)))))

(fn ConstructionScript
  (|CallParentFunction))