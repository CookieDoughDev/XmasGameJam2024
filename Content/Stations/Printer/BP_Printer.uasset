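; BP_Printer is an interactable station that turns a required carried item into a printed letter.
; On Interact, it checks the carried object's class against RequiredItem, then makes the BP_Player it is attached to drop it.
; The item is destroyed and a BP_Letter spawns at the ShippingLetterSpawnPosition transform, ignoring collisions.
; The construction script only calls its parent.
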(event EventInteract
  (params (CarriedObject :type Actor%20Object%20Reference))
  (if (== (Utilities|GetClass CarriedObject) (Variables|Default|GetRequiredItem))
    (bind _asbp_player (Utilities|Casting|CastToBP_Player (Actor|GetAttachParentActor CarriedObject)))
    (Default|DropObject _asbp_player)
    (Actor|DestroyActor CarriedObject)
    (Game|SpawnActorfromClass "/Game/Interactables/BP_Letter.BP_Letter_C" (Transformation|GetWorldTransform (Variables|Default|GetShippingLetterSpawnPosition)) "AlwaysSpawn" "MultiplyWithRoot" 0 0)))

(fn ConstructionScript
  (|CallParentFunction))