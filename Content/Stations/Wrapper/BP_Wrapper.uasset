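; BP_Wrapper is a station that turns a toy carried by the player into a wrapped present.
; On Interact it finds the player through the carried object's attach parent and makes them drop it.
; If the object is a BP_BaseToy, it spawns a BP_WrappedPresent at the spawn position component, passing the toy's mesh as the wrapped gift, then destroys the toy.
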(event EventBeginPlay
  (|CallParentFunction) ; This node is disabled and will not be called.\nDrag off pins to build functionality.
)

(event Collision|EventActorBeginOverlap
  (params (OtherActor :type Actor%20Object%20Reference))
  (|CallParentFunction OtherActor) ; This node is disabled and will not be called.\nDrag off pins to build functionality.
)

(event EventTick
  (params (DeltaSeconds :type Float%20%28single-precision%29))
  (|CallParentFunction DeltaSeconds) ; This node is disabled and will not be called.\nDrag off pins to build functionality.
)

(event EventInteract
  (params (CarriedObject :type Actor%20Object%20Reference))
  (Utilities|IsValid CarriedObject
    (:Is%20Valid
      (bind _asbp_player (Utilities|Casting|CastToBP_Player (Actor|GetAttachParentActor CarriedObject)))
      (Default|DropObject _asbp_player)
      (bind _asbp_base_toy (Utilities|Casting|CastToBP_BaseToy CarriedObject))
      (bind _toymesh (Default|GetToyMesh _asbp_base_toy))
      (Game|SpawnActorfromClass "/Game/Carryables/BP_WrappedPresent.BP_WrappedPresent_C" (Math|Transform|MakeTransform (.location (Transformation|GetWorldTransform (Variables|Default|GetWrappedPresent%20Spawn%20Position))) "0, 0, 0" "1.000000,1.000000,1.000000") "Undefined" "MultiplyWithRoot" 0 _toymesh 0 0)
      (Actor|DestroyActor CarriedObject))))

(fn ConstructionScript
  (|CallParentFunction))